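; BP_TNT is an explosive actor that spawns a poof effect, plays a sound and destroys itself when anything overlaps its Box.
; Overlaps on the outer Sphere toggle PlayerEject, gating an AddForce on the third-person character's capsule during the explosion.
; That force is the TNT's negated world location, rather than a direction toward the player.
; Debug prints and an arrow show the flag and the line to the player.
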(event OnComponentBeginOverlap(Sphere)
  (params (OverlappedComponent :type Primitive%20Component%20Object%20Reference) (OtherActor :type Actor%20Object%20Reference) (OtherComp :type Primitive%20Component%20Object%20Reference) (OtherBodyIndex :type Integer) (bFromSweep :type Boolean) (SweepResult :type Hit%20Result%20Structure%20%28by%20ref%29))
  ;[0.1254 0.15 0.04291 0.5] Toggle "PlayerEject" based on Sphere
  (Variables|Default|SetPlayerEject true)
  (Development|PrintString (Utilities|String|ToString(Boolean) (Variables|Default|GetPlayerEject)) true true "(R=1.000000,G=0.000000,B=0.005084,A=1.000000)"))

(event OnComponentEndOverlap(Sphere)
  (params (OverlappedComponent :type Primitive%20Component%20Object%20Reference) (OtherActor :type Actor%20Object%20Reference) (OtherComp :type Primitive%20Component%20Object%20Reference) (OtherBodyIndex :type Integer))
  ;[0.1254 0.15 0.04291 0.5] Toggle "PlayerEject" based on Sphere
  (Variables|Default|SetPlayerEject false)
  (Development|PrintString (Utilities|String|ToString(Boolean) (Variables|Default|GetPlayerEject)) true true "(R=1.000000,G=0.013515,B=0.000000,A=1.000000)"))

(event OnComponentBeginOverlap(Box)
  (params (OverlappedComponent :type Primitive%20Component%20Object%20Reference) (OtherActor :type Actor%20Object%20Reference) (OtherComp :type Primitive%20Component%20Object%20Reference) (OtherBodyIndex :type Integer) (bFromSweep :type Boolean) (SweepResult :type Hit%20Result%20Structure%20%28by%20ref%29))
  ;[0.625 0.4815 0.2376 0.5] Explode action + NS
  (Niagara|SpawnSystematLocation "/Game/Particules/NS_Poof.NS_Poof" (Transformation|GetActorLocation))
  (CallFunction|EventExplode))

(event Custom|EventExplode
  (bind _defaultsceneroot (Variables|Default|GetDefaultSceneRoot))
  (bind _returnvalue (Transformation|GetWorldLocation _defaultsceneroot))
  ;[0.5052 0 0.007261 0.5] Explode Force
  (bind _returnvalue_2 (Actor|GetActorOfClass "/Game/Blueprints/BP_ThirdPersonCharacter.BP_ThirdPersonCharacter_C"))
  (Audio|PlaySound2D "/Game/SFX/collide.collide" 1.0 1.0 0.0 0 0)
  (Rendering|Debug|DrawDebugArrow _returnvalue (Transformation|GetActorLocation _returnvalue_2) 1e+01 "(R=0.000000,G=1.000000,B=0.000000,A=1.000000)" 5.0 5.0)
  (if (Variables|Default|GetPlayerEject)
    (Physics|AddForce (Variables|/Script/Engine.Character|GetCapsuleComponent _returnvalue_2) (* _returnvalue "-1.000000,-1.000000,-1.000000") "None" false))
  (Actor|DestroyActor))

(event EventBeginPlay
  ;[0.15 0.15 0.15 0.5] Camera Ignore
  (Collision|SetCollisionResponsetoChannel (Variables|Default|GetCube) "ECC_Camera" "ECR_Ignore"))

(fn ConstructionScript)