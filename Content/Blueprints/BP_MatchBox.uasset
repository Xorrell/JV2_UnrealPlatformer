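; BP_MatchBox is a matchbox pickup that gives the player more matchsticks.
; It slowly spins every tick and sets its mesh to ignore the Camera collision channel on BeginPlay.
; On overlap with BP_ThirdPersonCharacter, it adds to that character's MatchstickCount, plays a victory sound and destroys itself.
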(event EventBeginPlay
  (bind _matchbox (Variables|Default|GetMatchBox))
  ;[0.15 0.15 0.15 0.5] Camera Ignore
  (Collision|SetCollisionResponsetoChannel _matchbox "ECC_Camera" "ECR_Ignore")
  (Collision|SetCollisionResponsetoChannel _matchbox "ECC_Camera" "ECR_Ignore"))

(event Collision|EventActorBeginOverlap
  (params (OtherActor :type Actor%20Object%20Reference))
  ;[0.4783 0.2915 0.2703 0.5] +5 MatchStick for Player
  (bind _asbp_third_person_character (Utilities|Casting|CastToBP_ThirdPersonCharacter OtherActor))
  (Variables|/Game/Blueprints/BP_ThirdPersonCharacter.BP_ThirdPersonCharacter_C|SetMatchstickCount _asbp_third_person_character (+ (Variables|/Game/Blueprints/BP_ThirdPersonCharacter.BP_ThirdPersonCharacter_C|GetMatchstickCount _asbp_third_person_character) 5))
  (Audio|PlaySound2D "/Game/SFX/victory.victory" 1.0 1.0 0.0 0 0)
  (Actor|DestroyActor))

(event EventTick
  (params (DeltaSeconds :type Float%20%28single-precision%29))
  ;[0.15 0.15 0.15 0.5] Auto Rotate
  (Transformation|AddActorLocalRotation "0.000000,1.000000,0.000000" false false))

(fn ConstructionScript)