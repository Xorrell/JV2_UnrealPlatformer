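; BP_Fuse_Ignited is an ignited fuse actor that looks for gunpowder and poofs away if none is found.
; Overlapping a BP_Gunpowder only draws a debug arrow toward it and prints "should move", with no movement implemented.
; One second after BeginPlay it checks PowderFound, which this graph never sets, and if false spawns the NS_Poof Niagara effect and destroys itself.
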(event OnComponentBeginOverlap(Bound)
  (params (OverlappedComponent :type Primitive%20Component%20Object%20Reference) (OtherActor :type Actor%20Object%20Reference) (OtherComp :type Primitive%20Component%20Object%20Reference) (OtherBodyIndex :type Integer) (bFromSweep :type Boolean) (SweepResult :type Hit%20Result%20Structure%20%28by%20ref%29))
  ;[0.15 0.15 0.15 0.5] Detect Gunpowder Collision
  (bind _asbp_gunpowder (Utilities|Casting|CastToBP_Gunpowder OtherActor))
  (Rendering|Debug|DrawDebugArrow (Transformation|GetWorldLocation (Variables|Default|GetDefaultSceneRoot)) (Transformation|GetActorLocation _asbp_gunpowder) 1e+01 "(R=0.000000,G=1.000000,B=0.000000,A=1.000000)" 2.0 0.0)
  (Development|PrintString "should move" true true "(R=0.124345,G=1.000000,B=0.000000,A=1.000000)" 1.5))

(event Custom|EventTooLong
  ;[0.15 0 0 0.5] If no Gunpowder, destroy it
  (Niagara|SpawnSystematLocation "/Game/Particules/NS_Poof.NS_Poof" (Transformation|GetWorldLocation (Variables|Default|GetDefaultSceneRoot)) "0, 0, 0" "0.100000,0.100000,0.100000")
  (Development|PrintString "Poof" true true "(R=0.976673,G=1.000000,B=0.892291,A=1.000000)")
  (Actor|DestroyActor))

(event EventBeginPlay
  ;[0.15 0.1252 0.06066 0.5] Check if no Gunpowder for too long
  (Actor|GetActorOfClass "/Game/Blueprints/BP_Gunpowder.BP_Gunpowder_C")
  (Utilities|FlowControl|Delay 1.0)
  (Development|PrintString "Delay over" true true "(R=1.000000,G=0.000000,B=0.518163,A=1.000000)")
  (if (Variables|Default|GetPowderFound)
    (Development|PrintString "Stay" true true "(R=1.000000,G=0.000389,B=0.105171,A=1.000000)")
    (else
      (CallFunction|EventTooLong))))

(fn ConstructionScript)