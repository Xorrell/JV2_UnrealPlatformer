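; BP_Matchstick is a spinning matchstick pickup that the third-person character collects.
; It rotates a fixed step each Tick, independent of delta time, and sets its Cube and Sphere to ignore the Camera channel on BeginPlay.
; On overlap with BP_ThirdPersonCharacter, it increments that character's MatchstickCount, prints the new total and destroys itself.
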(event EventBeginPlay
  ;[0.15 0.15 0.15 0.5] Camera Ignore
  (Collision|SetCollisionResponsetoChannel (Variables|Default|Getcube) "ECC_Camera" "ECR_Ignore")
  (Collision|SetCollisionResponsetoChannel (Variables|Default|GetSphere) "ECC_Camera" "ECR_Ignore"))

(event Collision|EventActorBeginOverlap
  (params (OtherActor :type Actor%20Object%20Reference))
  ;[0.4783 0.2915 0.2703 0.5] +1 MatchStick for Player
  (bind _asbp_third_person_character (Utilities|Casting|CastToBP_ThirdPersonCharacter OtherActor))
  (bind _output_get (Variables|/Game/Blueprints/BP_ThirdPersonCharacter.BP_ThirdPersonCharacter_C|SetMatchstickCount _asbp_third_person_character (+ (Variables|/Game/Blueprints/BP_ThirdPersonCharacter.BP_ThirdPersonCharacter_C|GetMatchstickCount _asbp_third_person_character) 1)))
  (Development|PrintString (Utilities|String|ToString(Byte) _output_get) true true "(R=1.000000,G=0.869907,B=0.000000,A=1.000000)")
  (Actor|DestroyActor))

(event EventTick
  (params (DeltaSeconds :type Float%20%28single-precision%29))
  ;[0.15 0.15 0.15 0.5] Auto Rotate
  (Transformation|AddActorLocalRotation "0.000000,1.000000,0.000000" false false))

(fn ConstructionScript)